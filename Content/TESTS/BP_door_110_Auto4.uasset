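; BP_door_110_Auto4 is a test door Blueprint with a trigger box and a handle, apparently an unfinished automatic door.
; Entering the box caches the first-person character and, if the door is flagged closed, calls SetOverridePhysicsAsset.
; Tick records whether that character overlaps the box and the handle's world location.
; No logic here moves the door, changes the closed flag or uses the recorded values.
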(event OnComponentBeginOverlap(Box)
  (params (OverlappedComponent :type Primitive%20Component%20Object%20Reference) (OtherActor :type Actor%20Object%20Reference) (OtherComp :type Primitive%20Component%20Object%20Reference) (OtherBodyIndex :type Integer) (bFromSweep :type Boolean) (SweepResult :type Hit%20Result%20Structure%20%28by%20ref%29))
  (bind _asbp_first_person_character (Utilities|Casting|CastToBP_FirstPersonCharacter OtherActor))
  (if (Variables|Default|GetISCLOSED)
    (Class|AnimNodeRigidBodyLibrary|SetOverridePhysicsAsset)))

(event EventTick
  (params (DeltaSeconds :type Float%20%28single-precision%29))
  (Variables|Default|SetOVERLAP (Collision|IsOverlappingActor (Variables|Default|GetBox) (stale OnComponentBeginOverlap(Box) _asbp_first_person_character) :!class /Script/Engine.PrimitiveComponent))
  (Variables|Default|SetLOCATION (Transformation|GetWorldLocation (Variables|Default|Gethandle))))

(fn ConstructionScript)