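; Test ceiling light actor that can flicker at random, with a point light and a mesh that swaps between lit and off materials.
; While flickering, Tick uses random delays to toggle the light, randomizing its intensity each time it turns on.
; If initially off, BeginPlay darkens it and binds a Light_switch click to an event that only clears the on and flickering flags.
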(event Custom|Turn%20off%20lights
  (params (TouchedActor :type Actor%20Object%20Reference) (ButtonPressed :type Key%20Structure :default "None"))
  (Variables|Default|SetIS%20ON false)
  (Variables|Default|SetIS%20FLICKERING false))

(event EventBeginPlay
  (if (not (Variables|Default|GetIS%20ON))
    (Rendering|Components|Light|SetIntensity (Variables|Default|GetPointLight) 0.0)
    (Rendering|Material|SetMaterial (Variables|Default|GetStaticMesh) 0 "/Game/TESTS/MAT_ceiling_off.MAT_ceiling_off")
    (Actor|GetAllActorsOfClass "/Game/TESTS/Light_switch.Light_switch_C")
    (bind _aslight_switch (Utilities|Casting|CastToLight_switch))
    (EventDispatchers|BindEventtoOnClicked _aslight_switch (delegate Custom|Turn%20off%20lights))))

(event EventTick
  (params (DeltaSeconds :type Float%20%28single-precision%29))
  (bind _pointlight (Variables|Default|GetPointLight))
  (bind _staticmesh (Variables|Default|GetStaticMesh))
  (if (Variables|Default|GetIS%20FLICKERING)
    (Utilities|FlowControl|Delay (Math|Random|RandomFloatinRange 0.002 0.5))
    (if (Variables|Default|GetIS%20ON)
      (Rendering|Components|Light|SetIntensity _pointlight 0.0)
      (Rendering|Material|SetMaterial _staticmesh 0 "/Game/TESTS/MAT_ceiling_off.MAT_ceiling_off")
      (Variables|Default|SetIS%20ON false)
      (else
        (Rendering|Components|Light|SetIntensity _pointlight (Math|Random|RandomFloatinRange 5e+02 7e+03))
        (Rendering|Material|SetMaterial _staticmesh 0 "/Game/TESTS/MAT_ceiling_light.MAT_ceiling_light")
        (Variables|Default|SetIS%20ON true)))))

(fn ConstructionScript)