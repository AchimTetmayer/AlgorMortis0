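; Office chair actor whose five base meshes, apparently caster wheels, swivel to face the direction the chair moves.
; The construction script adds the meshes in a ring and attaches them to the Empty component.
; Each Tick, when Box velocity on X or Y exceeds a small positive threshold, every child of Empty takes the velocity's world yaw, with zero pitch and roll.
; The threshold compares signed values, so movement purely toward negative axes leaves them unturned.
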(event EventTick
  (params (DeltaSeconds :type Float%20%28single-precision%29))
  (bind _box (Variables|Default|GetBox))
  (bind _returnvalue (Transformation|GetComponentVelocity _box))
  (bind _output_get (Variables|Default|SetIs%20Moving (or (> (.x _returnvalue) 1e+01) (> (.y _returnvalue) 1e+01))))
  (if _output_get
    (for _array_element (Components|GetChildrenComponents (Variables|Default|Getempty) false)
      (Transformation|SetWorldRotation _array_element (Math|Rotator|MakeRotator 0.0 0.0 (- (.Yaw (Math|Vector|GetYawPitchfromVector (Math|Vector|MakeVector (.x _returnvalue) (.y _returnvalue) (.z _returnvalue)))) 0.0)) false false))))

(fn ConstructionScript
  (bind _empty (Variables|Default|Getempty))
  (bind _returnvalue (AddComponent|AddStaticMeshComponent false (Math|Transform|MakeTransform (Math|Vector|MakeVector 25.0 -8.0 9.0) "0, 0, 0" "1.000000,1.000000,1.000000")))
  (bind _returnvalue_2 (AddComponent|AddStaticMeshComponent false (Math|Transform|MakeTransform (Math|Vector|MakeVector 0.0 -27.0 9.0) "0, 0, 0" "1.000000,1.000000,1.000000")))
  (bind _returnvalue_3 (AddComponent|AddStaticMeshComponent false (Math|Transform|MakeTransform (Math|Vector|MakeVector -25.0 -8.0 9.0) "0, 0, 0" "1.000000,1.000000,1.000000")))
  (bind _returnvalue_4 (AddComponent|AddStaticMeshComponent false (Math|Transform|MakeTransform (Math|Vector|MakeVector -15.0 21.0 9.0) "0, 0, 0" "1.000000,1.000000,1.000000")))
  (bind _returnvalue_5 (AddComponent|AddStaticMeshComponent false (Math|Transform|MakeTransform (Math|Vector|MakeVector 15.0 21.0 9.0) "0, 0, 0" "1.000000,1.000000,1.000000")))
  (Transformation|AttachComponentToComponent _returnvalue _empty "None" "KeepRelative" "KeepRelative" "KeepRelative" true)
  (Transformation|AttachComponentToComponent _returnvalue_2 _empty "None" "KeepRelative" "KeepRelative" "KeepRelative" true)
  (Transformation|AttachComponentToComponent _returnvalue_3 _empty "None" "KeepRelative" "KeepRelative" "KeepRelative" true)
  (Transformation|AttachComponentToComponent _returnvalue_4 _empty "None" "KeepRelative" "KeepRelative" "KeepRelative" true)
  (Transformation|AttachComponentToComponent _returnvalue_5 _empty "None" "KeepRelative" "KeepRelative" "KeepRelative" true))