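; BP_iv is an environment prop, likely a rolling IV stand, with four selectable heights.
; The construction script attaches four meshes in a cross under Empty and uses Type to position Top and Base and size the Box collision.
; Each tick, those child meshes swivel like casters to the yaw of Box's velocity, but only when its X or Y velocity exceeds a positive threshold.
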(event EventTick
  (params (DeltaSeconds :type Float%20%28single-precision%29))
  (bind _box (Variables|Default|GetBox))
  (bind _returnvalue (Transformation|GetComponentVelocity _box))
  (bind _output_get (Variables|Default|Setis%20moving (or (> (.x _returnvalue) 1e+01) (> (.y _returnvalue) 1e+01))))
  (if _output_get
    (for _array_element (Components|GetChildrenComponents (Variables|Default|Getempty) false)
      (Transformation|SetWorldRotation _array_element (Math|Rotator|MakeRotator 0.0 0.0 (- (.Yaw (Math|Vector|GetYawPitchfromVector (Math|Vector|MakeVector (.x _returnvalue) (.y _returnvalue) (.z _returnvalue)))) 0.0)) false false))))

(fn ConstructionScript
  (bind _empty (Variables|Default|Getempty))
  (bind _type (Variables|Default|Gettype))
  (bind _box (Variables|Default|GetBox))
  (bind _returnvalue (Utilities|Select :Index _type :Option%200 6e+01 :Option%201 75.0 :Option%202 9e+01 :Option%203 105.0))
  (bind _returnvalue_2 (AddComponent|AddStaticMeshComponent false (Math|Transform|MakeTransform (Math|Vector|MakeVector 0.0 -28.0 6.0) "0, 0, 0" "1.000000,1.000000,1.000000")))
  (bind _returnvalue_3 (AddComponent|AddStaticMeshComponent false (Math|Transform|MakeTransform (Math|Vector|MakeVector 0.0 28.0 6.0) "0, 0, 0" "1.000000,1.000000,1.000000")))
  (bind _returnvalue_4 (AddComponent|AddStaticMeshComponent false (Math|Transform|MakeTransform (Math|Vector|MakeVector 28.0 0.0 6.0) "0, 0, 0" "1.000000,1.000000,1.000000")))
  (bind _returnvalue_5 (AddComponent|AddStaticMeshComponent false (Math|Transform|MakeTransform (Math|Vector|MakeVector -28.0 0.0 6.0) "0, 0, 0" "1.000000,1.000000,1.000000")))
  (Transformation|AttachComponentToComponent _returnvalue_2 _empty "None" "KeepRelative" "KeepRelative" "KeepRelative" true)
  (Transformation|AttachComponentToComponent _returnvalue_3 _empty "None" "KeepRelative" "KeepRelative" "KeepRelative" true)
  (Transformation|AttachComponentToComponent _returnvalue_4 _empty "None" "KeepRelative" "KeepRelative" "KeepRelative" true)
  (Transformation|AttachComponentToComponent _returnvalue_5 _empty "None" "KeepRelative" "KeepRelative" "KeepRelative" true)
  (Transformation|SetRelativeLocation (Variables|Default|Gettop) (Math|Vector|MakeVector 0.0 0.0 (Utilities|Select :Index _type :Option%200 2e+01 :Option%201 5e+01 :Option%202 8e+01 :Option%203 1.1e+02)) false false)
  (Transformation|SetRelativeLocation _box (Math|Vector|MakeVector 0.0 0.0 _returnvalue) false false)
  (Components|Box|SetBoxExtent _box (Math|Vector|MakeVector 18.0 18.0 _returnvalue) true)
  (Transformation|SetRelativeLocation (Variables|Default|Getbase) (Math|Vector|MakeVector 0.0 0.0 (* _returnvalue -1.0)) false false))