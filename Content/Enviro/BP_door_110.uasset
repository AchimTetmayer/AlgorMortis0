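; Sliding door that opens automatically when the first-person character enters its Box trigger and closes when they leave.
; A Timeline lerps the Door's relative Y position, playing after a short delay to open and reversing at normal rate to close.
; The player's crouch or sprint state scales opening speed and sound volume, with sounds played at the Handle.
; Tick caches the Handle's world location, and an ISCLOSING flag tracks closing.
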(event OnComponentBeginOverlap(Box)
  (params (OverlappedComponent :type Primitive%20Component%20Object%20Reference) (OtherActor :type Actor%20Object%20Reference) (OtherComp :type Primitive%20Component%20Object%20Reference) (OtherBodyIndex :type Integer) (bFromSweep :type Boolean) (SweepResult :type Hit%20Result%20Structure%20%28by%20ref%29))
  (bind _asbp_first_person_character (Utilities|Casting|CastToBP_FirstPersonCharacter OtherActor))
  (Utilities|FlowControl|Delay 0.2)
  (Audio|PlaySoundatLocation "/Game/Sounds/Assets/DOORWood_Wooden_Barn_Door_Sliding_Doors_Open_Close_PSE_GEN3_GyaWj.DOORWood_Wooden_Barn_Door_Sliding_Doors_Open_Close_PSE_GEN3_GyaWj" (Transformation|GetWorldLocation (Variables|Default|Gethandle)) "0, 0, 0" (Math|Float|SelectFloat 0.2 (Math|Float|SelectFloat 2.0 1.0 (Variables|/Game/BP_FirstPersonCharacter.BP_FirstPersonCharacter_C|GetIS%20SPRINTING _asbp_first_person_character)) (Variables|/Game/BP_FirstPersonCharacter.BP_FirstPersonCharacter_C|GetIS%20CROUCHING _asbp_first_person_character)) 1.0 0.0 0 0 0 0)
  (Components|Timeline|SetPlayRate (Variables|Default|GetTimeline) (Math|Float|SelectFloat 1.0 (Math|Float|SelectFloat 4.0 2.0 (Variables|/Game/BP_FirstPersonCharacter.BP_FirstPersonCharacter_C|GetIS%20SPRINTING _asbp_first_person_character)) (Variables|/Game/BP_FirstPersonCharacter.BP_FirstPersonCharacter_C|GetIS%20CROUCHING _asbp_first_person_character)))
  (bind _newtrack_0 (Timeline|Timeline Play)
    (:Update
      (Transformation|SetRelativeLocation (Variables|Default|Getdoor) (Math|Vector|MakeVector 0.0 (Math|Float|Lerp -55.0 -155.0 _newtrack_0) 0.0) false false))
    (:Finished
      (if (stale OnComponentEndOverlap(Box) _output_get)
        (Variables|Default|SetISCLOSING false)))))

(event OnComponentEndOverlap(Box)
  (params (OverlappedComponent :type Primitive%20Component%20Object%20Reference) (OtherActor :type Actor%20Object%20Reference) (OtherComp :type Primitive%20Component%20Object%20Reference) (OtherBodyIndex :type Integer))
  (Utilities|Casting|CastToBP_FirstPersonCharacter OtherActor)
  (Components|Timeline|SetPlayRate (Variables|Default|GetTimeline) 1.0)
  (bind _output_get (Variables|Default|SetISCLOSING true))
  (Audio|PlaySoundatLocation "/Game/Sounds/Assets/DOORWood_Wooden_Barn_Door_Sliding_Doors_Open_Close_PSE_GEN3_GyaWj1.DOORWood_Wooden_Barn_Door_Sliding_Doors_Open_Close_PSE_GEN3_GyaWj1" (Transformation|GetWorldLocation (Variables|Default|Gethandle)) "0, 0, 0" 1.0 1.0 0.0 0 0 0 0)
  (bind _newtrack_0 (Timeline|Timeline Reverse)
    (:Update
      (Transformation|SetRelativeLocation (Variables|Default|Getdoor) (Math|Vector|MakeVector 0.0 (Math|Float|Lerp -55.0 -155.0 _newtrack_0) 0.0) false false))
    (:Finished
      (if _output_get
        (Variables|Default|SetISCLOSING false)))))

(event EventTick
  (params (DeltaSeconds :type Float%20%28single-precision%29))
  (Variables|Default|SetWOLOCATION (Transformation|GetWorldLocation (Variables|Default|Gethandle))))

(fn ConstructionScript)