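; Ceiling light actor that can start on or off, optionally flickers, and shuts off when a light switch is clicked.
; Each state change sets the rect light intensity, mesh material and audio volume together.
; Tick re-binds to the first found Light_switch's ONCLICK every frame and drives flicker through a random Delay with randomized on-intensity.
; The click handler only turns the light off and ends flickering, with no toggle back on.
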(event Custom|CustomEvent
  (Variables|Default|SetIS%20ON false)
  (Variables|Default|SetIS%20FLICKERING false)
  (Rendering|Components|Light|SetIntensity (Variables|Default|GetRectLight) 0.0)
  (Rendering|Material|SetMaterial (Variables|Default|GetStaticMesh) 0 "/Game/Enviro/MAT_ceiling_off.MAT_ceiling_off")
  (Audio|Components|Audio|SetVolumeMultiplier (Variables|Default|GetAudio) 0.0 :!class /Script/Engine.AudioComponent))

(event EventBeginPlay
  (bind _rectlight (Variables|Default|GetRectLight))
  (bind _staticmesh (Variables|Default|GetStaticMesh))
  (bind _audio (Variables|Default|GetAudio))
  (if (Variables|Default|GetIS%20ON)
    (Rendering|Components|Light|SetIntensity _rectlight 2.5e+03)
    (Rendering|Material|SetMaterial _staticmesh 0 "/Game/Enviro/MAT_ceiling_light.MAT_ceiling_light")
    (Audio|Components|Audio|SetVolumeMultiplier _audio 1.0 :!class /Script/Engine.AudioComponent)
    (else
      (Rendering|Components|Light|SetIntensity _rectlight 0.0)
      (Rendering|Material|SetMaterial _staticmesh 0 "/Game/Enviro/MAT_ceiling_off.MAT_ceiling_off")
      (Audio|Components|Audio|SetVolumeMultiplier _audio 0.0 :!class /Script/Engine.AudioComponent))))

(event EventTick
  (params (DeltaSeconds :type Float%20%28single-precision%29))
  (bind _staticmesh (Variables|Default|GetStaticMesh))
  (bind _audio (Variables|Default|GetAudio))
  (bind _rectlight (Variables|Default|GetRectLight))
  (bind _outactors (Actor|GetAllActorsOfClass "/Game/Enviro/Light_switch.Light_switch_C"))
  (EventDispatchers|BindEventtoONCLICK (Utilities|Array|Get(acopy) _outactors) (delegate Custom|CustomEvent))
  (if (Variables|Default|GetIS%20FLICKERING)
    (Utilities|FlowControl|Delay (Math|Random|RandomFloatinRange 0.002 0.5))
    (if (Variables|Default|GetIS%20ON)
      (Rendering|Components|Light|SetIntensity _rectlight 0.0)
      (Rendering|Material|SetMaterial _staticmesh 0 "/Game/Enviro/MAT_ceiling_off.MAT_ceiling_off")
      (Variables|Default|SetIS%20ON false)
      (Audio|Components|Audio|SetVolumeMultiplier _audio 0.0 :!class /Script/Engine.AudioComponent)
      (else
        (Rendering|Components|Light|SetIntensity _rectlight (Math|Random|RandomFloatinRange 5e+02 1e+03))
        (Rendering|Material|SetMaterial _staticmesh 0 "/Game/Enviro/MAT_ceiling_light.MAT_ceiling_light")
        (Variables|Default|SetIS%20ON true)
        (Audio|Components|Audio|SetVolumeMultiplier _audio 1.0 :!class /Script/Engine.AudioComponent)))))

(fn ConstructionScript)