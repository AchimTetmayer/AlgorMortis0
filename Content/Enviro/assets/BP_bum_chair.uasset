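; BP_bum_chair is an environment chair prop that characters can step up on only while it is roughly upright.
; On BeginPlay it adds a random world yaw to the Chair component, so each instance faces a different direction.
; Every Tick it checks the Chair's world roll and pitch, enabling CanCharacterStepUpOn within 45 degrees of level and disabling it otherwise.
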(event EventTick
  (params (DeltaSeconds :type Float%20%28single-precision%29))
  (bind _chair (Variables|Default|Getchair))
  (bind _chair_2 (Variables|Default|Getchair))
  (bind _returnvalue (Transformation|GetWorldRotation _chair))
  (if (and (and (> (.roll _returnvalue) -45.0) (< (.roll _returnvalue) 45.0)) (and (> (.pitch _returnvalue) -45.0) (< (.pitch _returnvalue) 45.0)))
    (Variables|/Script/Engine.PrimitiveComponent|SetCanCharacterStepUpOn _chair_2 "ECB_Yes")
    (else
      (Variables|/Script/Engine.PrimitiveComponent|SetCanCharacterStepUpOn _chair_2 "ECB_No"))))

(event EventBeginPlay
  (Transformation|AddWorldRotation (Variables|Default|Getchair) (Math|Rotator|MakeRotator 0.0 0.0 (.yaw (Math|Random|RandomRotator false))) false false))

(fn ConstructionScript)