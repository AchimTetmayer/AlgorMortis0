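; Industrial shelf environment prop that randomizes its own placement when play begins.
; BeginPlay adds a slight random yaw to the root component, then lowers it by a random stepped distance plus a small fixed offset.
; The construction script is empty, so the variation happens only at runtime.
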(event EventBeginPlay
  (Transformation|AddLocalRotation (Variables|Default|GetDefaultSceneRoot) (Math|Rotator|MakeRotator 0.0 0.0 (Math|Random|RandomFloatinRange -4.0 4.0)) false false)
  (bind _output_get (Variables|Default|Setbase%20location (Transformation|GetWorldLocation (Variables|Default|GetDefaultSceneRoot))))
  (Transformation|SetWorldLocation (Variables|Default|GetDefaultSceneRoot) (Math|Vector|MakeVector (.x _output_get) (.y _output_get) (+ (.z _output_get) (* (+ (* (Math|Random|RandomIntegerinRange 0 5) 50) 10) -1))) false false))

(fn ConstructionScript)