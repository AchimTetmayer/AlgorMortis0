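; Base enemy character that provides a melee attack, a patrol route and movement speed control.
; Attack plays a bash montage at increased rate and calls the AttackEnd dispatcher whether the montage completes or is interrupted.
; GetPatrolRoute exposes the stored route, while SetMovementSpeed maps a speed state from idle to sprinting onto the character's max walk speed and returns it.
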(event Custom|Attack
  (Animation|Montage|PlayMontage (Variables|Character|GetMesh) "/Game/Enemies/Till/Animations/Montage_Bash.Montage_Bash" 1.5
    (:OnCompleted
      _)
    (:OnInterrupted
      _))
  (Default|CallAttackEnd))

(fn ConstructionScript)

(fn GetPatrolRoute
  (return (Variables|AI|GetPatrolRoute)))

(fn SetMovementSpeed
  (params (Speed :type E_MovementSpeed%20Enum :default "NewEnumerator0"))
  (bind _output_get (Variables|/Script/Engine.CharacterMovementComponent|SetMaxWalkSpeed (Variables|Character|GetCharacterMovement) (Utilities|Select :Index Speed :NewEnumerator0 0.0 :NewEnumerator1 2e+02 :NewEnumerator2 3.5e+02 :NewEnumerator3 5e+02)))
  (return _output_get))